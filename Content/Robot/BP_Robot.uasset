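; BP_Robot is a robot Blueprint that reacts once to an Interact event.
; On the first interaction it plays a button-click sound in 2D, plays a non-looping animation on its Mesh and sets IsDead to true.
; A DoOnce blocks repeat interactions, and the BeginPlay, overlap and Tick events are disabled placeholders.
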(event EventBeginPlay
  (|CallParentFunction) ; This node is disabled and will not be called.\nDrag off pins to build functionality.
)

(event Collision|EventActorBeginOverlap
  (params (OtherActor :type Actor%20Object%20Reference))
  (|CallParentFunction OtherActor) ; This node is disabled and will not be called.\nDrag off pins to build functionality.
)

(event EventTick
  (params (DeltaSeconds :type Float%20%28single-precision%29))
  (|CallParentFunction DeltaSeconds) ; This node is disabled and will not be called.\nDrag off pins to build functionality.
)

(event EventInteract
  (Utilities|FlowControl|DoOnce false
    (:Completed
      (Audio|PlaySound2D "/Engine/VREditor/Sounds/UI/Click_on_Button_Cue.Click_on_Button_Cue" 1e+01 1.0 0.0 0 0)
      (Components|Animation|PlayAnimation (Variables|Character|GetMesh) 0 false)
      (Variables|Default|SetisDead true))))

(fn ConstructionScript
  (|CallParentFunction))