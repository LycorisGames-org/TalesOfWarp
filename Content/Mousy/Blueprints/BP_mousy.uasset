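; Enemy mouse that roams around its start point, chases pawns it senses in clear line of sight, and ends the game on touching the player.
; Interact kills it once, with a prompt shown while the player is nearby.
; The construction script builds a procedural vision-cone mesh from fanned traces, with optional bisection edge refinement.
; The cone uses unclipped trace ends, so walls don't shorten it, and it isn't rebuilt during play.
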(event OnSeePawn(childSensing)
  (params (Pawn :type Pawn%20Object%20Reference))
  (Utilities|FlowControl|Sequence
    (:then_0
      (if (not (Variables|Default|GetisDead))
        (bind _returnvalue (Collision|LineTraceByChannel (Transformation|GetActorLocation) (Transformation|GetActorLocation Pawn) "TraceTypeQuery1" false (Utilities|Array|MakeArray Pawn) "None"))
        (if (not _returnvalue)
          (AI|AIMoveTo self "0, 0, 0" Pawn 5.0 false
            (:then
              (Utilities|FlowControl|DoOnce false
                (:Completed
                  (Audio|PlaySoundatLocation "/Game/Mousy/Audio/mario_fall.mario_fall" (Transformation|GetActorLocation) "0, 0, 0" 1.0 1.0 0.0 0 0 0 0)
                  (bind _asbp_first_person_character (Utilities|Casting|CastToBP_FirstPersonCharacter Pawn))
                  (Default|SpottedEvent _asbp_first_person_character))))))))
    (:then_1
      (Utilities|FlowControl|RetriggerableDelay 1.0)
      (Development|PrintString "lost"))))

(event OnComponentBeginOverlap(collisionVolume)
  (params (OverlappedComponent :type Primitive%20Component%20Object%20Reference) (OtherActor :type Actor%20Object%20Reference) (OtherComp :type Primitive%20Component%20Object%20Reference) (OtherBodyIndex :type Integer) (bFromSweep :type Boolean) (SweepResult :type Hit%20Result%20Structure%20%28by%20ref%29))
  (if (not (Variables|Default|GetisDead))
    (bind _asbp_first_person_character (Utilities|Casting|CastToBP_FirstPersonCharacter OtherActor))
    (Variables|/Game/FirstPerson/Blueprints/BP_FirstPersonCharacter.BP_FirstPersonCharacter_C|SetisCaught _asbp_first_person_character true)
    (Variables|Default|SetgotPlayer true)
    (Development|PrintText "got")
    (Default|GameOver _asbp_first_person_character)))

(event OnComponentBeginOverlap(buttonVolume)
  (params (OverlappedComponent :type Primitive%20Component%20Object%20Reference) (OtherActor :type Actor%20Object%20Reference) (OtherComp :type Primitive%20Component%20Object%20Reference) (OtherBodyIndex :type Integer) (bFromSweep :type Boolean) (SweepResult :type Hit%20Result%20Structure%20%28by%20ref%29))
  (Utilities|Casting|CastToBP_FirstPersonCharacter OtherActor)
  (if (Variables|Default|GetisDead)
    (Development|SetHiddeninGame (Variables|Default|GetturnOffInteract) true false)
    (else
      (Development|SetHiddeninGame (Variables|Default|GetturnOffInteract) false false))))

(event OnComponentEndOverlap(buttonVolume)
  (params (OverlappedComponent :type Primitive%20Component%20Object%20Reference) (OtherActor :type Actor%20Object%20Reference) (OtherComp :type Primitive%20Component%20Object%20Reference) (OtherBodyIndex :type Integer))
  (Utilities|Casting|CastToBP_FirstPersonCharacter OtherActor)
  (Development|SetHiddeninGame (Variables|Default|GetturnOffInteract) true false))

(event Custom|RandomRoam
  (if (not (Variables|Default|GetisDead))
    (if (Class|KismetMathLibrary|NotEqualExactlyVectorVector (Variables|Default|GetanchorPoint) "0, 0, 0")
      _
      (else
        (Variables|Default|SetanchorPoint (Transformation|GetActorLocation))))
    (AI|AIMoveTo self (.RandomLocation (AI|Navigation|GetRandomReachablePointinRadius (Variables|Default|GetanchorPoint) 1.5e+03 0 0)) 0 5.0 false
      (:OnSuccess
        (Utilities|FlowControl|Delay 5.0)
        (CallFunction|RandomRoam)))))

(event EventBeginPlay
  (CallFunction|RandomRoam))

(event Collision|EventActorBeginOverlap
  (params (OtherActor :type Actor%20Object%20Reference)))

(event EventTick
  (params (DeltaSeconds :type Float%20%28single-precision%29)))

(event EventInteract
  (Utilities|FlowControl|DoOnce false
    (:Completed
      (Components|Animation|PlayAnimation (Variables|Character|GetMesh) "/Game/Mousy/Animations/Death_From_Back_Headshot.Death_From_Back_Headshot" false)
      (Audio|PlaySoundatLocation "/Engine/EditorSounds/GamePreview/EndSimulate.EndSimulate" (Transformation|GetActorLocation) "0, 0, 0" 1.0 1.0 0.0 0 0 0 0)
      (Variables|Default|SetisDead true))))

(fn ConstructionScript
  (if (Variables|FieldOfVision|Debug|GetRebuild)
    _
    (else
      _))
  (CallFunction|Start)
  (CallFunction|LineTracing))

(fn Start
  (Utilities|FlowControl|Sequence
    (:then_0
      (bind _output_get (Variables|FieldOfVision|Auxilliary|SetNumberOfSections (Math|Float|Ceil (/ (* (Variables|FieldOfVision|Base|GetHalfAngle) 2.0) (Variables|FieldOfVision|Base|GetDeltaAngle)))))
      (Variables|FieldOfVision|Auxilliary|SetdAngle (/ (* (Variables|FieldOfVision|Base|GetHalfAngle) 2.0) _output_get)))
    (:then_1
      (Variables|FieldOfVision|Auxilliary|SetStartPoint (+ (Math|Vector|MakeVector 0.0 0.0 (- (Variables|FieldOfVision|Base|GetHeightOfCheck) 1e+02)) (Transformation|GetActorLocation))))
    (:then_2
      (Transformation|AddLocalOffset (Variables|Default|GetProceduralMesh) (Math|Vector|MakeVector 0.0 0.0 (- (Variables|FieldOfVision|Base|GetHeightOfShow) 1e+02)) false false))))

(fn LineTracing
  (bind _startpoint (Variables|FieldOfVision|Auxilliary|GetStartPoint))
  (for _index (range 0 (Variables|FieldOfVision|Auxilliary|GetNumberOfSections))
    (LocalVariables|SetL_CurrentAngle (- (* _index (Variables|FieldOfVision|Auxilliary|GetdAngle)) (Variables|FieldOfVision|Base|GetHalfAngle)))
    (if (not (Variables|Default|GetisDead))
      (bind _outhit (Collision|LineTraceByChannel _startpoint (+ _startpoint (* (Math|Vector|RotateVectorAroundAxis (Transformation|GetActorForwardVector) (LocalVariables|GetL_CurrentAngle) "0.000000,0.000000,1.000000") (Variables|FieldOfVision|Base|GetExternalRadius))) "TraceTypeQuery1" false 0 (Variables|FieldOfVision|Debug|GetDraw%20Debug%20Type) true "(R=1.000000,G=0.000000,B=0.000000,A=1.000000)" "(R=0.000000,G=1.000000,B=0.000000,A=1.000000)" (Variables|FieldOfVision|Debug|GetDraw%20Time)))
      (Utilities|Array|Add (Variables|FieldOfVision|Auxilliary|GetHitResult) _outhit)))
  (if (Variables|FieldOfVision|Base|GetbUseExternalPrecise)
    (CallFunction|PreciseExternalBorders))
  (bind _index_2 (Utilities|FlowControl|ForLoopwithBreak 0 (- (Utilities|Array|LastIndex (Variables|FieldOfVision|Auxilliary|GetHitResult)) 1) :!label _label)
    (:LoopBody
      (if (Variables|Default|GetisDead)
        (CallFunction|Update)
        (Rendering|SetVisibility (Variables|Default|GetProceduralMesh) false false)
        (goto _label Break)
        (else
          (LocalVariables|Seti _index_2)
          (Utilities|FlowControl|Sequence
            (:then_0
              (if (.bBlockingHit (Collision|BreakHitResult (Utilities|Array|Get(acopy) (Variables|FieldOfVision|Auxilliary|GetHitResult) (LocalVariables|Geti))))
                (LocalVariables|SetL_LeftPoint (.Location (Collision|BreakHitResult (Utilities|Array|Get(acopy) (Variables|FieldOfVision|Auxilliary|GetHitResult) (LocalVariables|Geti)))))
                (else
                  (LocalVariables|SetL_LeftPoint (.TraceEnd (Collision|BreakHitResult (Utilities|Array|Get(acopy) (Variables|FieldOfVision|Auxilliary|GetHitResult) (LocalVariables|Geti)))))))
              (Variables|Alternate|SetalternateLeftNoCollision (.TraceEnd (Collision|BreakHitResult (Utilities|Array|Get(acopy) (Variables|FieldOfVision|Auxilliary|GetHitResult) (LocalVariables|Geti))))))
            (:then_1
              (if (.bBlockingHit (Collision|BreakHitResult (Utilities|Array|Get(acopy) (Variables|FieldOfVision|Auxilliary|GetHitResult) (+ (LocalVariables|Geti) 1))))
                (LocalVariables|SetL_RightPoint (.Location (Collision|BreakHitResult (Utilities|Array|Get(acopy) (Variables|FieldOfVision|Auxilliary|GetHitResult) (+ (LocalVariables|Geti) 1)))))
                (else
                  (LocalVariables|SetL_RightPoint (.TraceEnd (Collision|BreakHitResult (Utilities|Array|Get(acopy) (Variables|FieldOfVision|Auxilliary|GetHitResult) (+ (LocalVariables|Geti) 1)))))))
              (Variables|Alternate|SetalternateRightNoCollision (.TraceEnd (Collision|BreakHitResult (Utilities|Array|Get(acopy) (Variables|FieldOfVision|Auxilliary|GetHitResult) (+ (LocalVariables|Geti) 1))))))
            (:then_2
              (Class|ProceduralMeshComponent|CreateMeshSectionLinearColor (Variables|Default|GetProceduralMesh) (LocalVariables|Geti) (Utilities|Array|MakeArray (- (Variables|FieldOfVision|Auxilliary|GetStartPoint) (Variables|FieldOfVision|Auxilliary|GetStartPoint)) (- (Variables|Alternate|GetalternateLeftNoCollision) (Variables|FieldOfVision|Auxilliary|GetStartPoint)) (- (Variables|Alternate|GetalternateRightNoCollision) (Variables|FieldOfVision|Auxilliary|GetStartPoint))) (Utilities|Array|MakeArray 0 2 1) 0 0 0 0 0 0 0 false false)
              (Rendering|Material|SetMaterial (Variables|Default|GetProceduralMesh) (LocalVariables|Geti) "/Game/Mousy/Materials/m_instance.m_instance"))))))
    (:Completed
      (Transformation|SetRelativeRotation (Variables|Default|GetProceduralMesh) (* (Math|Rotator|MakeRotfromX (Transformation|GetActorForwardVector)) -1.0) false false))))

(fn Update
  (Variables|FieldOfVision|Auxilliary|SetStartPoint (+ (Math|Vector|MakeVector 0.0 0.0 (- (Variables|FieldOfVision|Base|GetHeightOfCheck) 1e+02)) (Transformation|GetActorLocation)))
  (Utilities|Array|Clear (Variables|FieldOfVision|Auxilliary|GetHitResult))
  (Class|ProceduralMeshComponent|ClearAllMeshSections (Variables|Default|GetProceduralMesh)))

(fn PreciseExternalBorders
  (for _index (range 0 (- (Utilities|Array|LastIndex (Variables|FieldOfVision|Auxilliary|GetHitResult)) 1))
    (LocalVariables|Seti _index)
    (Utilities|Array|Add (LocalVariables|GetL_HitResults) (Utilities|Array|Get(acopy) (Variables|FieldOfVision|Auxilliary|GetHitResult) (LocalVariables|Geti)))
    (if (!= (.HitActor (Collision|BreakHitResult (Utilities|Array|Get(acopy) (Variables|FieldOfVision|Auxilliary|GetHitResult) (LocalVariables|Geti)))) (.HitActor (Collision|BreakHitResult (Utilities|Array|Get(acopy) (Variables|FieldOfVision|Auxilliary|GetHitResult) (+ (LocalVariables|Geti) 1)))))
      (Utilities|FlowControl|Sequence
        (:then_0
          (if (.bBlockingHit (Collision|BreakHitResult (Utilities|Array|Get(acopy) (Variables|FieldOfVision|Auxilliary|GetHitResult) (LocalVariables|Geti))))
            (LocalVariables|SetL_LeftPoint (.Location (Collision|BreakHitResult (Utilities|Array|Get(acopy) (Variables|FieldOfVision|Auxilliary|GetHitResult) (LocalVariables|Geti)))))
            (else
              (LocalVariables|SetL_LeftPoint (.TraceEnd (Collision|BreakHitResult (Utilities|Array|Get(acopy) (Variables|FieldOfVision|Auxilliary|GetHitResult) (LocalVariables|Geti))))))))
        (:then_1
          (if (.bBlockingHit (Collision|BreakHitResult (Utilities|Array|Get(acopy) (Variables|FieldOfVision|Auxilliary|GetHitResult) (+ (LocalVariables|Geti) 1))))
            (LocalVariables|SetL_RightPoint (.Location (Collision|BreakHitResult (Utilities|Array|Get(acopy) (Variables|FieldOfVision|Auxilliary|GetHitResult) (+ (LocalVariables|Geti) 1)))))
            (else
              (LocalVariables|SetL_RightPoint (.TraceEnd (Collision|BreakHitResult (Utilities|Array|Get(acopy) (Variables|FieldOfVision|Auxilliary|GetHitResult) (+ (LocalVariables|Geti) 1))))))))
        (:then_2
          (bind _outhits (CallFunction|BisectionMethod (LocalVariables|GetL_LeftPoint) (LocalVariables|GetL_RightPoint) (Variables|FieldOfVision|Auxilliary|GetStartPoint) (.HitActor (Collision|BreakHitResult (Utilities|Array|Get(acopy) (Variables|FieldOfVision|Auxilliary|GetHitResult) (LocalVariables|Geti)))) (.HitActor (Collision|BreakHitResult (Utilities|Array|Get(acopy) (Variables|FieldOfVision|Auxilliary|GetHitResult) (+ (LocalVariables|Geti) 1))))))
          (for _array_element _outhits
            (Utilities|Array|Add (LocalVariables|GetL_HitResults) _array_element))))))
  (Utilities|Array|Add (LocalVariables|GetL_HitResults) (Utilities|Array|Get(acopy) (Variables|FieldOfVision|Auxilliary|GetHitResult) (Utilities|Array|LastIndex (Variables|FieldOfVision|Auxilliary|GetHitResult))))
  (Variables|FieldOfVision|Auxilliary|SetHitResult (LocalVariables|GetL_HitResults)))

(fn BisectionMethod
  (params (LeftPoint :type Vector) (RightPoint :type Vector) (StartPoint :type Vector) (LeftActor :type Actor%20Object%20Reference) (RightActor :type Actor%20Object%20Reference))
  (bind _returnvalue (- RightPoint StartPoint))
  (bind _l_otheractors (LocalVariables|GetL_OtherActors))
  ;[1 1 1] InitializeLocalVariables
  (LocalVariables|SetL_LeftDirection (- LeftPoint StartPoint))
  (LocalVariables|SetL_RightDirection _returnvalue)
  (LocalVariables|SetL_StartPoint StartPoint)
  (LocalVariables|SetL_LeftActor LeftActor)
  (LocalVariables|SetL_RightActor RightActor)
  (LocalVariables|SetL_CurrentAngle (Variables|FieldOfVision|Base|GetPreciseAngle) :!label _label)
  (LocalVariables|Setcount 0)
  (while (and (<= (Variables|FieldOfVision|Base|GetPreciseAngle) (LocalVariables|GetL_CurrentAngle)) (<= (LocalVariables|Getcount) (Variables|FieldOfVision|Debug|GetPreciseCount)))
    (Math|Integer|IncrementInt (LocalVariables|Getcount)
      (:%20%20
        (LocalVariables|SetL_CurrentAngle (Math|Float|Absolute(Float) (* (- (.Yaw (Math|Rotator|BreakRotator (Math|Rotator|MakeRotfromX (LocalVariables|GetL_LeftDirection)))) (.Yaw (Math|Rotator|BreakRotator (Math|Rotator|MakeRotfromX (LocalVariables|GetL_RightDirection))))) 0.5)))
        (LocalVariables|SetL_MidDirection (* (Math|Vector|Normalize (+ (Math|Vector|Normalize (LocalVariables|GetL_LeftDirection)) (Math|Vector|Normalize (LocalVariables|GetL_RightDirection)))) (Variables|FieldOfVision|Base|GetExternalRadius)))
        (bind _outhit (Collision|LineTraceByChannel (Variables|FieldOfVision|Auxilliary|GetStartPoint) (+ (Variables|FieldOfVision|Auxilliary|GetStartPoint) (LocalVariables|GetL_MidDirection)) "TraceTypeQuery1" false 0 "None"))
        (if (== (LocalVariables|GetL_LeftActor) (.HitActor (Collision|BreakHitResult _outhit)))
          (LocalVariables|SetL_LeftDirection (LocalVariables|GetL_MidDirection))
          (else
            (if (== (LocalVariables|GetL_RightActor) (.HitActor (Collision|BreakHitResult _outhit)))
              _
              (else
                (Utilities|Array|Insert (LocalVariables|GetL_OtherActors) (.HitActor (Collision|BreakHitResult _outhit)))))
            (LocalVariables|SetL_RightDirection (LocalVariables|GetL_MidDirection)))))))
  (bind _outhit_2 (Collision|LineTraceByChannel (LocalVariables|GetL_StartPoint) (+ (LocalVariables|GetL_StartPoint) (LocalVariables|GetL_LeftDirection)) "TraceTypeQuery1" false 0 (Variables|FieldOfVision|Debug|GetDraw%20Debug%20Type) true "(R=0.000000,G=0.000000,B=1.000000,A=1.000000)" "(R=0.000000,G=1.000000,B=1.000000,A=1.000000)" (Variables|FieldOfVision|Debug|GetDraw%20Time)))
  (Utilities|Array|Add (LocalVariables|GetL_NewHits) _outhit_2)
  (bind _outhit_3 (Collision|LineTraceByChannel (LocalVariables|GetL_StartPoint) (+ (LocalVariables|GetL_StartPoint) (LocalVariables|GetL_RightDirection)) "TraceTypeQuery1" false 0 (Variables|FieldOfVision|Debug|GetDraw%20Debug%20Type) true "(R=0.000000,G=0.000000,B=1.000000,A=1.000000)" "(R=0.000000,G=1.000000,B=1.000000,A=1.000000)" (Variables|FieldOfVision|Debug|GetDraw%20Time)))
  (Utilities|Array|Add (LocalVariables|GetL_NewHits) _outhit_3)
  (if (!= (Utilities|Array|Length _l_otheractors) 0)
    (LocalVariables|SetL_LeftActor (Utilities|Array|Get(acopy) _l_otheractors))
    (Utilities|Array|RemoveIndex (LocalVariables|GetL_OtherActors))
    (LocalVariables|SetL_LeftDirection (LocalVariables|GetL_RightDirection))
    (LocalVariables|SetL_RightDirection _returnvalue)
    (goto _label)
    (else
      (return (LocalVariables|GetL_NewHits)))))