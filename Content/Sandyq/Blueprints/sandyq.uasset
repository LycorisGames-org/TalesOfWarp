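; Interactable puzzle actor (sandyq, a chest) that yields a statue key once its puzzle is finished.
; It caches the overlapping BP_FirstPersonCharacter, and Interact calls SolveGolovolomka (puzzle) on that player.
; finishGolovolomka destroys the actor and spawns a BP_StatueKey slightly above its location, adding a rotating movement component at runtime to spin the key.
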(event Custom|finishGolovolomka
  (Actor|DestroyActor)
  (bind _returnvalue (Game|SpawnActorfromClass "/Game/ThrowMaterial/MechaKey/BP_StatueKey.BP_StatueKey_C" (Math|Conversions|ToTransform(Vector) (+ (Transformation|GetActorLocation) "0.000000,0.000000,80.000000")) "Undefined" 0 0))
  (bind _returnvalue_2 (AddComponent|AddRotatingMovementComponent _returnvalue))
  (Variables|/Script/Engine.RotatingMovementComponent|SetPivotTranslation _returnvalue_2 "0.000000,0.000000,1.000000")
  (Variables|/Script/Engine.RotatingMovementComponent|SetRotationRate _returnvalue_2 "0.000000,60.000000,0.000000"))

(event EventBeginPlay)

(event Collision|EventActorBeginOverlap
  (params (OtherActor :type Actor%20Object%20Reference))
  (bind _asbp_first_person_character (Utilities|Casting|CastToBP_FirstPersonCharacter OtherActor))
  (Variables|Default|SetplayerRef _asbp_first_person_character))

(event EventTick
  (params (DeltaSeconds :type Float%20%28single-precision%29)))

(event EventInteract
  (Default|SolveGolovolomka (Variables|Default|GetplayerRef)))

(fn ConstructionScript)